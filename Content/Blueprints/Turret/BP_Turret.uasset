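; BP_Turret is a turret that turns to face the player character and shoots at it.
; Each PawnSensing sighting of a BP_FPCharacter snaps the whole actor to a look-at rotation, then waits TimeToShoot before spawning a BP_Bullet at the right barrel.
; Sightings during the wait still update rotation but do not restart the Delay, which paces the fire.
; The left barrel transform is left unused.
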(event `self.PawnSensing.OnSeePawn`
  (params (Pawn :type "Pawn Object Reference"))
  (cast `/Game/Blueprints/Player/BP_FPCharacter` Pawn)
  (`self.K2_SetActorRotation` (`KismetMathLibrary.FindLookAtRotation` (`self.K2_GetActorLocation`) (`self.K2_GetActorLocation` Pawn)))
  (`KismetSystemLibrary.Delay` (`self.TimeToShoot`))
  (`|SpawnActorFromClass` "/Game/Blueprints/Turret/BP_Bullet.BP_Bullet_C" (`SceneComponent.K2_GetComponentToWorld` (`self.Right Barrel`)) "Undefined" "MultiplyWithRoot" null null))

(fn `UserConstructionScript`)